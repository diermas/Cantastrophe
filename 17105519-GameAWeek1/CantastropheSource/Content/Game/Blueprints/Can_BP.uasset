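; A timed can hazard that changes colour, fuses and explodes unless it first reaches a trigger on the floor.
; On BeginPlay its lifetime is derived from elapsed game time, so later cans have shorter fuses, and a timeline scaled to it tints the material.
; Chained delays start fuse audio and smoke halfway, then report the explosion to Floor_BP.
; Overlapping the trigger silences the fuse, destroys the can and reports a hit; physical hits play a sound.
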(event `self.ReceiveActorBeginOverlap`
  (params (OtherActor :type "Actor Object Reference"))
  ;[1 1 1] Code to run when a can hits the TriggerBox on the floor
  (if (== OtherActor (`self.Trigger`))
    (`ActorComponent.SetActive` (stale `self.ReceiveBeginPlay` _returnvalue_3) false false)
    (`self.K2_DestroyActor`)
    (bind _outactors (`GameplayStatics.GetAllActorsOfClass` "/Game/Game/Blueprints/Floor_BP.Floor_BP_C"))
    (`/Game/Game/Blueprints/Floor_BP.Canhit` (`|GetArrayItem` _outactors))))

(event `self.ReceiveBeginPlay`
  (bind _returnvalue_location (`KismetMathLibrary.BreakTransform` (`self.GetTransform`)))
  (bind _returnvalue (/ (- 30 (`KismetMathLibrary.FTrunc` (`KismetSystemLibrary.GetGameTimeInSeconds`))) 2))
  (bind _returnvalue_2 (/ _returnvalue 2))
  (`TimelineComponent.SetPlayRate` (`self.CanGradient`) (/ 10.0 (`KismetMathLibrary.Conv_IntToDouble` _returnvalue)))
  (bind (_direction _newtrack_0) (`Timeline|CanGradient`)
    (:`Update`
      (`MeshComponent.SetVectorParameterValueOnMaterials` (`self.Can`) "Can Colour" (`KismetMathLibrary.Conv_LinearColorToVector` _newtrack_0))
      ;[1 1 1] Code to play can audio
      (`KismetSystemLibrary.Delay` (`KismetMathLibrary.Conv_IntToDouble` _returnvalue_2))
      (bind _returnvalue_3 (`GameplayStatics.SpawnSoundAtLocation` "/Game/Game/Audio/FuseAudio.FuseAudio" (`self.K2_GetActorLocation`)))
      (`GameplayStatics.SpawnEmitterAttached` "/Game/Game/Particles/Smoke_PS.Smoke_PS" (`self.Can`) "None" _returnvalue_location (struct) (1.0 1.0 1.0) "KeepWorldPosition")
      (`KismetSystemLibrary.Delay` (`KismetMathLibrary.Conv_IntToDouble` _returnvalue_2))
      (`ActorComponent.SetActive` _returnvalue_3 false false)
      (bind _outactors (`GameplayStatics.GetAllActorsOfClass` "/Game/Game/Blueprints/Floor_BP.Floor_BP_C"))
      (`/Game/Game/Blueprints/Floor_BP.Canexploded` (`|GetArrayItem` _outactors)))))

(event `self.ReceiveHit`
  (params (MyComp :type "PrimitiveComponent Object Reference") (Other :type "Actor Object Reference") (OtherComp :type "PrimitiveComponent Object Reference") (bSelfMoved :type Boolean) (HitLocation :type "Vector Structure") (HitNormal :type "Vector Structure") (NormalImpulse :type "Vector Structure") (Hit :type "HitResult Structure (by ref)"))
  ;[1 1 1] Can Hit Sound Trigger
  (`GameplayStatics.PlaySoundAtLocation` "/Game/Game/Audio/CanHitAudio.CanHitAudio" HitLocation))

(fn `UserConstructionScript`)